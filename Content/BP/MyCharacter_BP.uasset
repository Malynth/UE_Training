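; Player character Blueprint with axis-driven movement and look, a standard jump, and pick-up-and-carry of physics objects.
; Movement follows control yaw; an alternative timeline-driven jump that sets actor height is left unconnected.
; Pressing Use traces from the camera for PhysicsBody objects, with persistent debug drawing, and grabs the hit component with a PhysicsHandle.
; Tick keeps the handle target a fixed distance ahead of the camera until Use is released.
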(event `InputAxis|MoveForward`
  (params (AxisValue :type "Float (single-precision)"))
  (bind (_returnvalue_roll _returnvalue_pitch _returnvalue_yaw) (`KismetMathLibrary.BreakRotator` (`self.GetControlRotation`)))
  ;[1 1 1] Movement
  (`self.AddMovementInput` (`KismetMathLibrary.GetForwardVector` (`KismetMathLibrary.MakeRotator` 0.0 0.0 _returnvalue_yaw)) AxisValue))

(event `InputAxis|MoveRight`
  (params (AxisValue :type "Float (single-precision)"))
  (bind (_returnvalue_roll _returnvalue_pitch _returnvalue_yaw) (`KismetMathLibrary.BreakRotator` (`self.GetControlRotation`)))
  ;[1 1 1] Movement
  (`self.AddMovementInput` (`KismetMathLibrary.GetRightVector` (`KismetMathLibrary.MakeRotator` 0.0 0.0 _returnvalue_yaw)) AxisValue))

(event `InputAxis|LookUp`
  (params (AxisValue :type "Float (single-precision)"))
  ;[1 1 1] Looking
  (`self.AddControllerPitchInput` AxisValue))

(event `InputAxis|LookRight`
  (params (AxisValue :type "Float (single-precision)"))
  ;[1 1 1] Looking
  (`self.AddControllerYawInput` AxisValue))

(event `InputAction|Jump`
  (params (Key :type "Key Structure")))

(event `InputAction|Jump`
  (params (Key :type "Key Structure"))
  (:`Pressed`
    (`self.Jump`)))

(event `self.ReceiveTick`
  (params (DeltaSeconds :type "Float (single-precision)"))
  (bind _playercameramanager (`PlayerController.PlayerCameraManager` (`GameplayStatics.GetPlayerController` 0)))
  (`PhysicsHandleComponent.SetTargetLocation` (`self.PhysicsHandle`) (+ (`PlayerCameraManager.GetCameraLocation` _playercameramanager) (* (`KismetMathLibrary.Normal` (`KismetMathLibrary.GetForwardVector` (`PlayerCameraManager.GetCameraRotation` _playercameramanager))) 150))))

(event `InputAction|Use`
  (params (Key :type "Key Structure"))
  (bind _playercameramanager (`PlayerController.PlayerCameraManager` (`GameplayStatics.GetPlayerController` 0)))
  (bind _returnvalue (`PlayerCameraManager.GetCameraLocation` _playercameramanager))
  (:`Pressed`
    (bind _outhit (`KismetSystemLibrary.LineTraceSingleForObjects` :`Start` _returnvalue :`End` (+ _returnvalue (* (`KismetMathLibrary.Normal` (`KismetMathLibrary.GetForwardVector` (`PlayerCameraManager.GetCameraRotation` _playercameramanager))) (`self.Use Distance`))) :`ObjectTypes` (`|MakeArray` "ObjectTypeQuery4" :!type "EObjectTypeQuery Enum") :`DrawDebugType` "Persistent"))
    (if (`GameplayStatics.BreakHitResult` _outhit)
      (`PhysicsHandleComponent.GrabComponentAtLocationWithRotation` (`self.PhysicsHandle`) (`.HitComponent` (`GameplayStatics.BreakHitResult` _outhit)) "None" (`.Location` (`GameplayStatics.BreakHitResult` _outhit)) (`self.K2_GetActorRotation` (`ActorComponent.GetOwner` (`.HitComponent` (`GameplayStatics.BreakHitResult` _outhit)))))))
  (:`Released`
    (`PhysicsHandleComponent.ReleaseComponent` (`self.PhysicsHandle`))))

(fn `UserConstructionScript`)